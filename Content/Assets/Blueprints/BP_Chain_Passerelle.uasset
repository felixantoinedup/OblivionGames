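; Footbridge chain actor that drops its chain with a falling-chain sound the first time anything overlaps its trigger box.
; The overlap enables chain physics and runs a timeline that offsets the chain, destroying it ten seconds after the timeline finishes.
; A delay inside the timeline update calls PullChains on BP_Chaines_tirées actors.
; A camera look-at sequence with input lock is present but disconnected.
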(event OnComponentBeginOverlap(TriggerBox)
  (params (OverlappedComponent :type Primitive%20Component%20Object%20Reference) (OtherActor :type Actor%20Object%20Reference) (OtherComp :type Primitive%20Component%20Object%20Reference) (OtherBodyIndex :type Integer) (bFromSweep :type Boolean) (SweepResult :type Hit%20Result%20Structure%20%28by%20ref%29))
  ;[1 1 1] Prog de Base de triggerbox et mouvement
  (Utilities|FlowControl|DoOnce false
    (:Completed
      (Audio|PlaySound2D "/Game/Assets/Sounds/SFX_FallingChain_Cue.SFX_FallingChain_Cue")
      (Physics|SetSimulatePhysics (Variables|Default|GetChain) true)
      (bind _newtrack_0 (Timeline|Timeline_0 Play)
        (:Update
          (Transformation|AddLocalOffset (Variables|Default|GetChain) (+ (Math|Conversions|ToVector(Float) _newtrack_0) "0.000000,50.000000,0.000000") false false)
          (Utilities|FlowControl|Delay 2.5)
          (bind _outactors (Actor|GetAllActorsOfClass "/Game/Assets/Blueprints/BP_Chaines_tirées.BP_Chaines_tirées_C"))
          (Default|PullChains _outactors))
        (:Finished
          (Utilities|FlowControl|Delay 1e+01)
          (Components|DestroyComponent (Variables|Default|GetChain)))))))

(fn ConstructionScript)