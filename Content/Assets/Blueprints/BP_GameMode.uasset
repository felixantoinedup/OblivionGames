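; BP_GameMode is a game mode Blueprint that sets up the UI and intro sound when play begins.
; BeginPlay creates the BP_UserInterface widget, adds it to the viewport, then plays a gate-closing 2D sound from a late start offset.
; OnDeathEvent is an empty stub.
; Respawn experiments, including a temporary level reload and several RestartPlayer variants, are left disconnected and never run.
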(event Custom|OnDeathEvent
  ;[1 1 1] On death event
)

(event EventBeginPlay
  ;[1 1 1] ON GAME BEGIN
  ;;[1 1 1] Intro Animation handling
  (Utilities|FlowControl|Sequence
    (:then_0
      (bind _returnvalue (UserInterface|CreateWidget "/Game/Assets/Blueprints/MenuAndUI/BP_UserInterface.BP_UserInterface_C"))
      (UserInterface|Viewport|AddtoViewport _returnvalue 0))
    (:then_1
      (Audio|PlaySound2D "/Game/Assets/Sounds/INTRO__GateClosing_Cue.INTRO__GateClosing_Cue" 6.0 1.0 10.35))))

(fn ConstructionScript)