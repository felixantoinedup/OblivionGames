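; BP_SlowWalk is a trigger volume that slows the player's walking speed while something overlaps it.
; TriggerBox begin and end overlap call SlowDownCharacter and CharacterNormalSpeed, which subtract and add back a fixed offset on MaxWalkSpeed.
; Both functions fetch player 0 as BP_Character and edit its CharacterMovementComponent, without checking which actor overlapped, so any overlap alters the player's speed and multiple overlaps stack.
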(event OnComponentBeginOverlap(TriggerBox)
  (params (OverlappedComponent :type Primitive%20Component%20Object%20Reference) (OtherActor :type Actor%20Object%20Reference) (OtherComp :type Primitive%20Component%20Object%20Reference) (OtherBodyIndex :type Integer) (bFromSweep :type Boolean) (SweepResult :type Hit%20Result%20Structure%20%28by%20ref%29))
  ;[1 1 1] Character Movement affected by Triggerbox
  (CallFunction|SlowDownCharacter))

(event OnComponentEndOverlap(TriggerBox)
  (params (OverlappedComponent :type Primitive%20Component%20Object%20Reference) (OtherActor :type Actor%20Object%20Reference) (OtherComp :type Primitive%20Component%20Object%20Reference) (OtherBodyIndex :type Integer))
  ;[1 1 1] Character Movement affected by Triggerbox
  (CallFunction|CharacterNormalSpeed))

(fn ConstructionScript)

(fn SlowDownCharacter
  (bind _asbp_character (Utilities|Casting|CastToBP_Character (Game|GetPlayerCharacter 0)))
  (bind _ascharacter_movement_component (Utilities|Casting|CastToCharacterMovementComponent (Pawn|GetMovementComponent _asbp_character)))
  (Variables|/Script/Engine.CharacterMovementComponent|SetMaxWalkSpeed _ascharacter_movement_component (- (Variables|/Script/Engine.CharacterMovementComponent|GetMaxWalkSpeed _ascharacter_movement_component) 2e+02)))

(fn CharacterNormalSpeed
  (bind _asbp_character (Utilities|Casting|CastToBP_Character (Game|GetPlayerCharacter 0)))
  (bind _ascharacter_movement_component (Utilities|Casting|CastToCharacterMovementComponent (Pawn|GetMovementComponent _asbp_character)))
  (Variables|/Script/Engine.CharacterMovementComponent|SetMaxWalkSpeed _ascharacter_movement_component (+ (Variables|/Script/Engine.CharacterMovementComponent|GetMaxWalkSpeed _ascharacter_movement_component) 2e+02)))