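; BP_Altar is a one-use altar that grants the player character an electricity charge.
; A one-shot trigger plays a lightning strike with flashes and sound, then lights the altar with particles and an endlessly randomized flickering light.
; While activatable, its interaction trigger calls UIAltar on the user interface widget.
; CE_PlayAltarActions hides the lit effects, disables reactivation and increments the character's ElectricityCharge.
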(event OnComponentBeginOverlap(TriggerLightning)
  (params (OverlappedComponent :type Primitive%20Component%20Object%20Reference) (OtherActor :type Actor%20Object%20Reference) (OtherComp :type Primitive%20Component%20Object%20Reference) (OtherBodyIndex :type Integer) (bFromSweep :type Boolean) (SweepResult :type Hit%20Result%20Structure%20%28by%20ref%29))
  (bind _pointlight_lit_altar (Variables|Default|GetPointLight_lit_Altar))
  (Utilities|FlowControl|DoOnce false
    (:Completed
      ;[1 1 1] Lightning Animation
      (Utilities|FlowControl|Sequence
        (:then_0
          (Development|SetHiddeninGame (Variables|Default|GetLightningPlane) false false)
          (Utilities|FlowControl|Delay 0.1)
          (Development|SetHiddeninGame (Variables|Default|GetLightningPlane) true false)
          (Utilities|FlowControl|Delay 0.1)
          (Development|SetHiddeninGame (Variables|Default|GetLightningPlane) false false)
          (Utilities|FlowControl|Delay 0.1)
          (Development|SetHiddeninGame (Variables|Default|GetLightningPlane) true false))
        (:then_1
          (Audio|PlaySound2D "/Game/Assets/Sounds/SFX_LightningStrike_Cue.SFX_LightningStrike_Cue")
          (Development|SetHiddeninGame _pointlight_lit_altar false false)
          (Rendering|Components|Light|SetIntensity _pointlight_lit_altar (Math|Random|RandomFloatinRange 0.0 1e+07) :!label _label)
          (Utilities|FlowControl|Delay 0.05)
          (goto _label))
        (:then_2
          (Development|SetHiddeninGame (Variables|Default|GetParticleSystem) false false))))))

(event OnComponentBeginOverlap(TriggerCanInteract)
  (params (OverlappedComponent :type Primitive%20Component%20Object%20Reference) (OtherActor :type Actor%20Object%20Reference) (OtherComp :type Primitive%20Component%20Object%20Reference) (OtherBodyIndex :type Integer) (bFromSweep :type Boolean) (SweepResult :type Hit%20Result%20Structure%20%28by%20ref%29))
  ;[1 1 1] If colliding with player pawn AND altar is activatable
  (if (and (== (Utilities|GetClass OtherActor) "/Game/Assets/Blueprints/BP_Character.BP_Character_C") (Variables|Default|GetisActivatable))
    ;[1 1 1] Do UI stuff
    (bind _foundwidgets (Widget|GetAllWidgetsOfClass "/Game/Assets/Blueprints/MenuAndUI/BP_UserInterface.BP_UserInterface_C" true))
    (for _array_element _foundwidgets
      (Default|UIAltar _array_element))))

(event OnComponentEndOverlap(TriggerCanInteract)
  (params (OverlappedComponent :type Primitive%20Component%20Object%20Reference) (OtherActor :type Actor%20Object%20Reference) (OtherComp :type Primitive%20Component%20Object%20Reference) (OtherBodyIndex :type Integer))
  ;[1 1 1] If player pawn leaves collider
  (if (and (== (Utilities|GetClass OtherActor) "/Game/Assets/Blueprints/BP_Character.BP_Character_C") (Variables|Default|GetisActivatable))
    _))

(event Custom|CE_PlayAltarActions
  (if (Variables|Default|GetisActivatable)
    (Development|SetHiddeninGame (Variables|Default|GetPointLight_lit_Altar) true false)
    (Development|SetHiddeninGame (Variables|Default|GetParticleSystem) true false)
    (Utilities|FlowControl|Sequence
      (:then_0
        (Variables|Default|SetisActivatable false))
      (:then_2
        ;[1 1 1] Increment electricity charge
        (bind _asbp_character (Utilities|Casting|CastToBP_Character (Game|GetPlayerCharacter 0)))
        (Variables|/Game/Assets/Blueprints/BP_Character.BP_Character_C|SetElectricityCharge _asbp_character (+ (Variables|/Game/Assets/Blueprints/BP_Character.BP_Character_C|GetElectricityCharge _asbp_character) 1))))))

(fn ConstructionScript)