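; Stalagmite platform Blueprint that falls under physics, meant to land on a lower platform.
; An arrow hit destroys the arrow, plays a fall sound and, through a DoOnce, enables physics on the stalagmite.
; After a short delay, the shatter pieces start simulating and the stalagmite stops, to prevent abuse.
; BeginPlay also jumps straight into this physics sequence, bypassing the hit check and DoOnce.
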(event OnComponentHit(SM_Stalagmite)
  (params (HitComponent :type Primitive%20Component%20Object%20Reference) (OtherActor :type Actor%20Object%20Reference) (OtherComp :type Primitive%20Component%20Object%20Reference) (NormalImpulse :type Vector :default "0, 0, 0") (Hit :type Hit%20Result%20Structure%20%28by%20ref%29))
  ;[1 1 1] Check if hit by an arrow class object
  (if (== (Utilities|GetClass OtherActor) "/Game/Assets/Blueprints/BP_Arrow.BP_Arrow_C")
    (Utilities|FlowControl|Sequence
      (:then_0
        (Actor|DestroyActor OtherActor))
      (:then_1
        (Utilities|FlowControl|DoOnce false
          (:Completed
            ;[1 1 1] Set simulate physics - for the object to fall on a lower platform
            (Physics|SetSimulatePhysics (Variables|Default|GetSM_Stalagmite) true)
            ;[1 1 1] Remove simulate physics for abuse-proof
            (Utilities|FlowControl|Delay 3.0)
            (Physics|SetSimulatePhysics (Variables|Default|GetLP_Stalashatter_LP_10) true) ; Make sure to lock the right rotation and position axises
            (Physics|SetSimulatePhysics (Variables|Default|GetSM_Stalagmite) false) ; Make sure to lock the right rotation and position axises
          )))
      (:then_2
        (Audio|PlaySoundatLocation "/Game/Assets/Sounds/SFX_StalagmiteFall_Cue.SFX_StalagmiteFall_Cue" (Transformation|GetWorldLocation (Variables|Default|GetSM_Stalagmite)))))))

(event EventBeginPlay
  ;[1 1 1] Set simulate physics - for the object to fall on a lower platform
  (Physics|SetSimulatePhysics (Variables|Default|GetSM_Stalagmite) true)
  ;[1 1 1] Remove simulate physics for abuse-proof
  (Utilities|FlowControl|Delay 3.0)
  (Physics|SetSimulatePhysics (Variables|Default|GetLP_Stalashatter_LP_10) true) ; Make sure to lock the right rotation and position axises
  (Physics|SetSimulatePhysics (Variables|Default|GetSM_Stalagmite) false) ; Make sure to lock the right rotation and position axises
)

(fn ConstructionScript)