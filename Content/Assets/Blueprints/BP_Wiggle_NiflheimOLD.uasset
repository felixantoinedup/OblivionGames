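; BP_Wiggle_NiflheimOLD is a trigger actor that nudges the player character upward when its TriggerBox is entered, apparently as a wiggle effect.
; Begin overlap calls CharacterWiggle, where a DoOnce with no reset plays a timeline once.
; Each update moves BP_Character toward 50 units above its current location, using the timeline float as VInterpTo's DeltaTime.
; End overlap teleports this actor itself to the character's location.
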(event OnComponentBeginOverlap(TriggerBox)
  (params (OverlappedComponent :type Primitive%20Component%20Object%20Reference) (OtherActor :type Actor%20Object%20Reference) (OtherComp :type Primitive%20Component%20Object%20Reference) (OtherBodyIndex :type Integer) (bFromSweep :type Boolean) (SweepResult :type Hit%20Result%20Structure%20%28by%20ref%29))
  ;[1 1 1] Character Movement
  (Variables|Default|SetPlayerInTriggerBox true)
  (CallFunction|CharacterWiggle))

(event OnComponentEndOverlap(TriggerBox)
  (params (OverlappedComponent :type Primitive%20Component%20Object%20Reference) (OtherActor :type Actor%20Object%20Reference) (OtherComp :type Primitive%20Component%20Object%20Reference) (OtherBodyIndex :type Integer))
  ;[1 1 1] Character Movement
  (Variables|Default|SetPlayerInTriggerBox false)
  (bind _asbp_character (Utilities|Casting|CastToBP_Character (Game|GetPlayerCharacter 0)))
  (Transformation|SetActorLocation (Transformation|GetActorLocation _asbp_character) false true))

(event Custom|Character%20Wiggle
  ;[1 1 1] Character Movement
  (if (Variables|Default|GetPlayerInTriggerBox)
    (bind _asbp_character (Utilities|Casting|CastToBP_Character (Game|GetPlayerCharacter 0)))
    (Utilities|FlowControl|DoOnce false
      (:Completed
        (bind _movement_float (Timeline|Timeline_0 Play)
          (:Update
            (Transformation|SetActorLocation _asbp_character (Math|Interpolation|VInterpTo (Transformation|GetActorLocation _asbp_character) (+ (Transformation|GetActorLocation _asbp_character) "0, 0,50.000000") _movement_float 3.0) false false)))))))

(fn ConstructionScript)