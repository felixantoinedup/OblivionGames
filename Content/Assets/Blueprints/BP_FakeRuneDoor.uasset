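; BP_FakeRuneDoor is a rune door Blueprint with a Box trigger that detects the player character entering and leaving its area.
; Both overlap events act only when the actor's class is exactly BP_Character and IsActivatable is true.
; The UI show and remove steps are placeholder debug prints, and the file contains no door-opening logic.
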(event OnComponentBeginOverlap(Box)
  (params (OverlappedComponent :type Primitive%20Component%20Object%20Reference) (OtherActor :type Actor%20Object%20Reference) (OtherComp :type Primitive%20Component%20Object%20Reference) (OtherBodyIndex :type Integer) (bFromSweep :type Boolean) (SweepResult :type Hit%20Result%20Structure%20%28by%20ref%29))
  ;[1 1 1] If colliding with player pawn AND rune is activatable
  (if (and (== (Utilities|GetClass OtherActor) "/Game/Assets/Blueprints/BP_Character.BP_Character_C") (Variables|Default|GetisActivatable))
    ;[1 1 1] Do UI stuff
    (Development|PrintString "Show UI")))

(event OnComponentEndOverlap(Box)
  (params (OverlappedComponent :type Primitive%20Component%20Object%20Reference) (OtherActor :type Actor%20Object%20Reference) (OtherComp :type Primitive%20Component%20Object%20Reference) (OtherBodyIndex :type Integer))
  ;[1 1 1] If player pawn leaves collider
  (if (and (== (Utilities|GetClass OtherActor) "/Game/Assets/Blueprints/BP_Character.BP_Character_C") (Variables|Default|GetisActivatable))
    ;[1 1 1] Remove UI stuff
    (Development|PrintString "Remove UI")))

(fn ConstructionScript)