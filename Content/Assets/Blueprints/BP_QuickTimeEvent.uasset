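; BP_QuickTimeEvent is an actor that starts a timed quick-time event when a BP_Character overlaps it.
; It enables input and compares each key press to a target key, either succeeding immediately or accumulating progress to 100 in mashable mode.
; Success pauses the timer and destroys the actor.
; Timeout disables input, resets progress and calls the game mode's death event; feedback is only printed strings, as the prompt text node is unconnected.
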(event Collision|EventActorBeginOverlap
  (params (OtherActor :type Actor%20Object%20Reference))
  ;[1 1 1] On collision with player, start QTE
  (CallFunction|QTEStart OtherActor))

(event Input|KeyboardEvents|AnyKey
  (params (Key :type Key%20Structure :default "AnyKey"))
  ;[1 1 1] Check if is correct input
  (:Pressed
    (if (== Key (Variables|Default|GetKey%20To%20Press))
      ;[1 1 1] If key is good, check if mashable or not
      (if (Variables|Default|GetisMashableQTE?)
        ;[1 1 1] Record QTE Progress
        (bind _output_get (Variables|Default|SetMashableQTEProgress (+ (Variables|Default|GetMashableQTEProgress) (Variables|Default|GetMashableQTEJumpProgress))))
        (if (>= _output_get 1e+02)
          (CallFunction|QTESuccess)
          (else
            (Development|PrintString (Utilities|String|ToString(Float) (Variables|Default|GetMashableQTEProgress)))))
        (else
          (CallFunction|QTESuccess)))
      (else
        ;[1 1 1] If key is wrong
        (Development|PrintString "wrongkey")))))

(fn ConstructionScript)

(fn QTEFail
  (Development|PrintString "FAILED")
  (Utilities|FlowControl|Sequence
    (:then_0
      ;[1 1 1] Stop listening to player inputs
      (Input|DisableInput (Game|GetPlayerController 0))
      (Variables|Default|SetMashableQTEProgress 0.0))
    (:then_1
      (bind _asbp_game_mode (Utilities|Casting|CastToBP_GameMode (Game|GetGameMode)))
      (Default|OnDeathEvent _asbp_game_mode))))

(fn QTEStart
  (params (Object :type Object%20Object%20Reference))
  (Utilities|Casting|CastToBP_Character Object)
  (Utilities|FlowControl|Sequence
    (:then_0
      ;[1 1 1] Start listening to player inputs
      (Input|EnableInput (Game|GetPlayerController 0)))
    (:then_1
      ;[1 1 1] Start a timer, If time runs out - call QTE_Fail()
      (Utilities|Time|SetTimerbyFunctionName 0 "QTE_Fail" (Variables|Default|GetQTE_TimeLimit))
      (Development|PrintString "QTE START"))))

(fn QTESuccess
  ;[1 1 1] Kill timer, kill actor
  (Class|KismetSystemLibrary|PauseTimer 0 "QTE_Fail")
  (Development|PrintString "WIN")
  (Actor|DestroyActor))