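; BP_FakeRuneDoor_02 is a rune door actor that costs the player electricity to activate, though its door motion is not wired up.
; Box overlaps with BP_Character print placeholder show/remove UI messages while IsActivatable is true.
; ActivateRuneDoor clears that flag, calls an empty play-actions event and decrements player 0's ElectricityCharge.
; Timelines for rotating two rotators and offsetting the root vertically exist but are never triggered.
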(event OnComponentBeginOverlap(Box)
  (params (OverlappedComponent :type Primitive%20Component%20Object%20Reference) (OtherActor :type Actor%20Object%20Reference) (OtherComp :type Primitive%20Component%20Object%20Reference) (OtherBodyIndex :type Integer) (bFromSweep :type Boolean) (SweepResult :type Hit%20Result%20Structure%20%28by%20ref%29))
  ;[1 1 1] If colliding with player pawn AND rune is activatable
  (if (and (== (Utilities|GetClass OtherActor) "/Game/Assets/Blueprints/BP_Character.BP_Character_C") (Variables|Default|GetisActivatable))
    ;[1 1 1] Do UI stuff
    (Development|PrintString "Show UI")))

(event OnComponentEndOverlap(Box)
  (params (OverlappedComponent :type Primitive%20Component%20Object%20Reference) (OtherActor :type Actor%20Object%20Reference) (OtherComp :type Primitive%20Component%20Object%20Reference) (OtherBodyIndex :type Integer))
  ;[1 1 1] If player pawn leaves collider
  (if (and (== (Utilities|GetClass OtherActor) "/Game/Assets/Blueprints/BP_Character.BP_Character_C") (Variables|Default|GetisActivatable))
    ;[1 1 1] Remove UI stuff
    (Development|PrintString "Remove UI")))

(event Custom|CE_PlayRuneDoorActions)

(fn ConstructionScript)

(fn ActivateRuneDoor
  (Utilities|FlowControl|Sequence
    (:then_0
      (Variables|Default|SetisActivatable false))
    (:then_1
      (CallFunction|CEPlayRuneDoorActions))
    (:then_2
      ;[1 1 1] Decrement electricity charge
      (bind _asbp_character (Utilities|Casting|CastToBP_Character (Game|GetPlayerCharacter 0)))
      (bind _output_get (Variables|/Game/Assets/Blueprints/BP_Character.BP_Character_C|SetElectricityCharge _asbp_character (- (Variables|/Game/Assets/Blueprints/BP_Character.BP_Character_C|GetElectricityCharge _asbp_character) 1)))
      (Development|PrintString (Utilities|String|ToString(Integer) _output_get)))))