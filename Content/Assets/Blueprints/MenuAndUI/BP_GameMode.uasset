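; Game mode Blueprint that sets up the user interface and runs the intro when play begins.
; BeginPlay adds BP_UserInterface to the viewport, then a sequence triggers its UI intro, the intro event on BP_Character and a gate-closing sound.
; The death event is empty, and the experimental respawn logic, including a temporary level reload and several RestartPlayer variants, is disconnected and never runs.
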(event Custom|OnDeathEvent
  ;[1 1 1] On death event
)

(event EventBeginPlay
  ;[1 1 1] ON GAME BEGIN
  (bind _returnvalue (UserInterface|CreateWidget "/Game/Assets/Blueprints/MenuAndUI/BP_UserInterface.BP_UserInterface_C"))
  (UserInterface|Viewport|AddtoViewport _returnvalue 0)
  ;;[1 1 1] Intro Animation handling
  ;; Unlink before the sequence
  ;; if you dont want the intro anim
  (Utilities|FlowControl|Sequence
    (:then_0
      (Default|UIIntro _returnvalue))
    (:then_1
      (bind _asbp_character (Utilities|Casting|CastToBP_Character (Game|Player|GetPlayerPawn 0)))
      (Default|CEIntro _asbp_character))
    (:then_2
      (Audio|PlaySound2D "/Game/Assets/Sounds/INTRO__GateClosing_Cue.INTRO__GateClosing_Cue" 6.0 1.0 10.35))))

(fn ConstructionScript)