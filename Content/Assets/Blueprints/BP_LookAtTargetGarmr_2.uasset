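; One-shot trigger volume that forces the player's view toward a look-at target, apparently for a Garmr moment.
; When BP_Character overlaps the box, it disables input and stores the controller's rotation.
; A timeline lerps control rotation along the shortest path to a look-at rotation recomputed each update, then restores input.
; The trigger also plays a growl, moves a particle component and prints placeholder animation text.
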(event OnComponentBeginOverlap(Box)
  (params (OverlappedComponent :type Primitive%20Component%20Object%20Reference) (OtherActor :type Actor%20Object%20Reference) (OtherComp :type Primitive%20Component%20Object%20Reference) (OtherBodyIndex :type Integer) (bFromSweep :type Boolean) (SweepResult :type Hit%20Result%20Structure%20%28by%20ref%29))
  (bind _returnvalue (Game|GetPlayerCharacter 0))
  (bind _returnvalue_2 (Game|GetPlayerController 0))
  (bind _lookattarget (Variables|Default|GetLookAtTarget))
  (bind _returnvalue_3 (Transformation|GetActorLocation _returnvalue_2))
  (bind _returnvalue_4 (Transformation|GetWorldLocation _lookattarget))
  (bind _returnvalue_5 (Math|Rotator|FindLookatRotation _returnvalue_3 _returnvalue_4))
  (bind (_roll _pitch _yaw) (Math|Rotator|BreakRotator _returnvalue_5))
  ;[1 1 1] If colliding with player pawn
  (if (== (Utilities|GetClass OtherActor) "/Game/Assets/Blueprints/BP_Character.BP_Character_C")
    (Utilities|FlowControl|DoOnce false
      (:Completed
        (Utilities|FlowControl|Sequence
          (:then_0
            (Input|DisableInput _returnvalue 0))
          (:then_1
            (Utilities|Casting|CastToBP_Character OtherActor)
            ;[1 1 1] Get player initial camera rotation (A)
            (Variables|Default|SetInitial%20Rotation (Transformation|GetActorRotation _returnvalue_2)) ; Store initial camera view
            (bind _rotationlerpalpha (Timeline|RotationLerpTimeline PlayFromStart) ; Animation for the camera for point A to B
              (:Update
                (Pawn|SetControlRotation _returnvalue_2 (Math|Rotator|Lerp(Rotator) (Variables|Default|GetInitial%20Rotation) (Math|Rotator|MakeRotator _roll _pitch _yaw) _rotationlerpalpha true)))
              (:Finished
                (Input|EnableInput _returnvalue 0))))
          (:then_2
            ;[1 1 1] Do more stuff
            (Development|PrintString "Hello")
            (Audio|PlaySound2D "/Game/Assets/Sounds/SFX_GarmGrowl_02_Cue.SFX_GarmGrowl_02_Cue")
            (Components|MoveComponentTo (Variables|Default|GetParticleSystem) "0, 0,10000.000000" "0, 0, 0" false false 0.2 false)
            (Development|PrintString "play anim")))))))

(fn ConstructionScript)