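; BP_Shadow is an actor with a hidden Shadow component that appears and slides away, apparently triggered by overlapping TestTriggerBox.
; Shadow is hidden at BeginPlay, and the overlap calls SpawnShadow, presumably the Spawn_Shadow event that unhides it.
; After a short delay, a timeline moves Shadow by a fixed local offset on each update without sweep, so distance depends on frame rate.
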(event OnComponentBeginOverlap(testTriggerBox)
  (params (OverlappedComponent :type Primitive%20Component%20Object%20Reference) (OtherActor :type Actor%20Object%20Reference) (OtherComp :type Primitive%20Component%20Object%20Reference) (OtherBodyIndex :type Integer) (bFromSweep :type Boolean) (SweepResult :type Hit%20Result%20Structure%20%28by%20ref%29))
  (CallFunction|SpawnShadow))

(event Custom|Spawn_Shadow
  (Development|SetHiddeninGame (Variables|Default|GetShadow) false false)
  (Utilities|FlowControl|Delay 2.0)
  (Timeline|Timeline_0 Play
    (:Update
      (Transformation|AddLocalOffset (Variables|Default|GetShadow) "-5.000000,2.000000,0.000000" false false))))

(event EventBeginPlay
  ;[1 1 1] hide at start
  (Development|SetHiddeninGame (Variables|Default|GetShadow) true false))

(fn ConstructionScript)