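; BP_LookAtTarget is a one-shot trigger volume that turns the player's view toward a target as a scripted moment with a growl and moving particles.
; When BP_Character overlaps the box outside its intro animation, input is disabled while a timeline lerps control rotation toward LookAtTarget, then restored.
; Alongside, a growl plays and a second timeline pushes the particle system along, which later deactivates before the actor destroys itself.
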(event OnComponentBeginOverlap(Box)
  (params (OverlappedComponent :type Primitive%20Component%20Object%20Reference) (OtherActor :type Actor%20Object%20Reference) (OtherComp :type Primitive%20Component%20Object%20Reference) (OtherBodyIndex :type Integer) (bFromSweep :type Boolean) (SweepResult :type Hit%20Result%20Structure%20%28by%20ref%29))
  (bind _returnvalue (Game|GetPlayerCharacter 0))
  (bind _returnvalue_2 (Game|GetPlayerController 0))
  (bind _lookattarget (Variables|Default|GetLookAtTarget))
  (bind _returnvalue_3 (Transformation|GetActorLocation _returnvalue_2))
  (bind _returnvalue_4 (Transformation|GetWorldLocation _lookattarget))
  (bind _returnvalue_5 (Math|Rotator|FindLookatRotation _returnvalue_3 _returnvalue_4))
  (bind (_roll _pitch _yaw) (Math|Rotator|BreakRotator _returnvalue_5))
  ;[1 1 1] If colliding with player pawn
  (bind _asbp_character (Utilities|Casting|CastToBP_Character OtherActor))
  (if (and (== (Utilities|GetClass OtherActor) "/Game/Assets/Blueprints/BP_Character.BP_Character_C") (not (Variables|/Game/Assets/Blueprints/BP_Character.BP_Character_C|GetIsInIntroAnimation _asbp_character)))
    (Utilities|FlowControl|DoOnce false
      (:Completed
        (Utilities|FlowControl|Sequence
          (:then_0
            (Input|DisableInput _returnvalue 0))
          (:then_1
            (Utilities|Casting|CastToBP_Character OtherActor)
            ;[1 1 1] Get player initial camera rotation (A)
            (Variables|Default|SetInitial%20Rotation (Transformation|GetActorRotation _returnvalue_2)) ; Store initial camera view
            (bind _rotationlerpalpha (Timeline|RotationLerpTimeline PlayFromStart) ; Animation for the camera for point A to B
              (:Update
                (Pawn|SetControlRotation _returnvalue_2 (Math|Rotator|Lerp(Rotator) (Variables|Default|GetInitial%20Rotation) (Math|Rotator|MakeRotator _roll _pitch _yaw) _rotationlerpalpha true)))
              (:Finished
                (Input|EnableInput _returnvalue 0))))
          (:then_2
            (Utilities|FlowControl|Sequence
              (:then_0
                (Audio|PlaySound2D "/Game/Assets/Sounds/SFX_GarmGrowl_01_Cue.SFX_GarmGrowl_01_Cue")
                (Components|Activation|Activate (Variables|Default|GetParticleSystem) false))
              (:then_1
                (Timeline|Timeline_0 Play
                  (:Update
                    (Transformation|AddLocalOffset (Variables|Default|GetParticleSystem) (Math|Vector|MakeVector 6e+02 -35.0 -3e+01) false false))))
              (:then_2
                (Utilities|FlowControl|Delay 4.0)
                (Components|Activation|Deactivate (Variables|Default|GetParticleSystem))
                (Utilities|FlowControl|Delay 1e+01)
                (Actor|DestroyActor)))))))))

(fn ConstructionScript)