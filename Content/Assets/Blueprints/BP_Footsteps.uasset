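; BP_Footsteps is an unfinished footstep Blueprint meant to track the stride of an owning Character.
; Tick first casts an unconnected input to BP_Character, then checks whether the owner has moved beyond Stride since LastFootstepsLocation while on the ground.
; A non-Character owner triggers a debug print.
; The passing branch ends at a second cast, leaving the downward-trace nodes unwired, with no sound or location update.
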(event EventTick
  (params (DeltaSeconds :type Float%20%28single-precision%29))
  ;[1 1 1] Tick
  (Utilities|Casting|CastToBP_Character)
  (bind _ascharacter (Utilities|Casting|CastToCharacter (Components|GetOwner))
    (:then
      (if (and (> (Math|Vector|VectorLength (- (Transformation|GetActorLocation (Components|GetOwner)) (Variables|Default|GetLastFootstepsLocation))) (Variables|Default|GetStride)) (AI|Components|NavMovement|IsMovingonGround (Pawn|GetMovementComponent _ascharacter)))
        (bind _ascharacter_2 (Utilities|Casting|CastToCharacter (Components|GetOwner)))))
    (:CastFailed
      (Development|PrintString "BP_FootstepsATTACHEDto noncharacterActor"))))

(fn ConstructionScript)