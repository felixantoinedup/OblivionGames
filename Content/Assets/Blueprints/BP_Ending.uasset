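; BP_Ending is the ending trigger actor that plays the game's final sequence around the collar chains.
; The first TriggerBox overlap tells the player's BP_Character to play its end animation.
; After timed delays it plays the Garmr scream, then slides the chains far along X from RestingLocation and reveals a particle system.
; The physics and timeline chain logic, which alone sets RestingLocation, is disconnected, and PullChain is empty.
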(event OnComponentBeginOverlap(TriggerBox)
  (params (OverlappedComponent :type Primitive%20Component%20Object%20Reference) (OtherActor :type Actor%20Object%20Reference) (OtherComp :type Primitive%20Component%20Object%20Reference) (OtherBodyIndex :type Integer) (bFromSweep :type Boolean) (SweepResult :type Hit%20Result%20Structure%20%28by%20ref%29))
  ;[1 1 1] Set Variable GAME ENDED on true (to disable input and play animation on BP_Character)
  (Utilities|FlowControl|DoOnce false
    (:Completed
      (bind _asbp_character (Utilities|Casting|CastToBP_Character (Game|Player|GetPlayerPawn 0)))
      (Default|CEPlayEndAnimation _asbp_character)
      (Utilities|FlowControl|Delay 5.5)
      ;[1 1 1] Play Ending
      (Audio|PlaySound2D "/Game/Assets/Sounds/ENDING_GarmrScream_Cue.ENDING_GarmrScream_Cue")
      (Utilities|FlowControl|Delay 1.0)
      (Utilities|FlowControl|Sequence
        (:then_0
          (Components|MoveComponentTo (Variables|Default|GetSM_Collar_Chains) (+ (Variables|Default|GetResting%20Location) "10000.000000, 0,0.000000") "0, 0, 0" false false 2.0 false))
        (:then_1
          (Development|SetHiddeninGame (Variables|Default|GetParticleSystem) false false))))))

(event EventBeginPlay
  ;[1 1 1] Give Chains nice pose
)

(fn ConstructionScript)

(fn PullChain)