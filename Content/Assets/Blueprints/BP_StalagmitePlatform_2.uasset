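; BP_StalagmitePlatform_2 is a stalagmite platform whose shatter and fall sequence plays once when CE_PlayStalagmiteActions is called.
; A DoOnce gates the event, then a fixed delay precedes the fall.
; It plays the AStalashatter animation while a timeline moves that component along Z, scaled by frame delta time, and plays a 2D fall sound.
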(event Custom|CE_PlayStalagmiteActions
  (Utilities|FlowControl|DoOnce false
    (:Completed
      (Utilities|FlowControl|Delay 4.2)
      (Utilities|FlowControl|Sequence
        (:then_0
          ;[1 1 1] Stalagmite fall aniatmion
          (Components|Animation|PlayAnimation (Variables|Default|GetA_Stalashatter) "/Game/Assets/Meshes/Props/Stalagmite/A_Stalashatter_Anim.A_Stalashatter_Anim" false)
          (bind _newtrack_0 (Timeline|Timeline_0 Play)
            (:Update
              (Transformation|AddLocalOffset (Variables|Default|GetA_Stalashatter) (Math|Vector|MakeVector 0.0 0.0 (* (* (.z _newtrack_0) 2.3) (Utilities|Time|GetWorldDeltaSeconds))) false false))))
        (:then_1
          (Audio|PlaySound2D "/Game/Assets/Sounds/SFX_StalagmiteFall_Cue.SFX_StalagmiteFall_Cue"))))))

(fn ConstructionScript)