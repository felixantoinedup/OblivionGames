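; BP_FogColorModifier is a trigger actor that blends a referenced fog actor to a new color and density when overlapped.
; Its Cube is visible for editing and hidden in game at BeginPlay.
; Any actor overlap stores the current inscattering color, then restarts a timeline that lerps color and density toward the target values.
; Density always blends from a hardcoded start value, and nothing reverts on exit.
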(event EventBeginPlay
  (Development|SetHiddeninGame (Variables|Default|GetCube) true false))

(event Collision|EventActorBeginOverlap
  (params (OtherActor :type Actor%20Object%20Reference))
  (bind _fog (Variables|Default|GetFog))
  (bind _component (Variables|/Script/Engine.ExponentialHeightFog|GetComponent _fog))
  (Variables|Default|SetOldColor (Variables|/Script/Engine.ExponentialHeightFogComponent|GetFogInscatteringColor _component))
  (bind _newtrack_0 (Timeline|lerp PlayFromStart)
    (:Update
      (Class|ExponentialHeightFogComponent|SetFogInscatteringColor _component (Math|Color|Lerp(LinearColor) (Variables|Default|GetOldColor) (Variables|Default|GetNewColor) _newtrack_0))
      (Class|ExponentialHeightFogComponent|SetFogDensity _component (Math|Float|Lerp 0.02 (Variables|Default|GetNewDensity) _newtrack_0)))))

(fn ConstructionScript)