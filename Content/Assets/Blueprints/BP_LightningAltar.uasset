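; Lightning altar actor that flashes lightning on overlap and can be interacted with to hide its particle effects.
; Entering the lightning trigger box flickers the initially hidden lightning component twice through timed visibility toggles.
; A second box sets an in-range flag, which is never cleared and does not check the overlapping actor.
; With that flag set, the Interact input hides two particle systems in sequence, half a second apart.
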(event OnComponentBeginOverlap(Box)
  (params (OverlappedComponent :type Primitive%20Component%20Object%20Reference) (OtherActor :type Actor%20Object%20Reference) (OtherComp :type Primitive%20Component%20Object%20Reference) (OtherBodyIndex :type Integer) (bFromSweep :type Boolean) (SweepResult :type Hit%20Result%20Structure%20%28by%20ref%29))
  (Variables|Default|SetPlayerInRangeOfActivating true))

(event OnComponentBeginOverlap(LightningTriggerBox)
  (params (OverlappedComponent :type Primitive%20Component%20Object%20Reference) (OtherActor :type Actor%20Object%20Reference) (OtherComp :type Primitive%20Component%20Object%20Reference) (OtherBodyIndex :type Integer) (bFromSweep :type Boolean) (SweepResult :type Hit%20Result%20Structure%20%28by%20ref%29))
  ;[1 1 1] Lightning Animation
  (Development|SetHiddeninGame (Variables|Default|GetlightningComponent) false false)
  (Utilities|FlowControl|Delay 0.1)
  (Development|SetHiddeninGame (Variables|Default|GetlightningComponent) true false)
  (Utilities|FlowControl|Delay 0.1)
  (Development|SetHiddeninGame (Variables|Default|GetlightningComponent) false false)
  (Utilities|FlowControl|Delay 0.1)
  (Development|SetHiddeninGame (Variables|Default|GetlightningComponent) true false))

(event EventBeginPlay
  (Development|SetHiddeninGame (Variables|Default|GetlightningComponent) true false))

(event Input|ActionEvents|InputActionInteract
  (params (Key :type Key%20Structure :default "AnyKey"))
  (:Pressed
    (if (Variables|Default|GetPlayerInRangeOfActivating)
      (Development|SetHiddeninGame (Variables|Default|GetParticleSystem1) true false)
      (Utilities|FlowControl|Delay 0.5)
      (Development|SetHiddeninGame (Variables|Default|GetParticleSystem) true false))))

(fn ConstructionScript)